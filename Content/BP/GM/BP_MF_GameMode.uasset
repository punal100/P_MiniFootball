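; BP_MF_GameMode is a game mode Blueprint whose only active logic is PostLogin calling its parent.
; BeginPlay, Tick and Event_Assign_To_Team are empty.
; Disconnected nodes hold a staggered team-assignment loop that would queue joining players in TempPlayers, assign each to the next available team, possess that team's first character, then repeat after a delay.
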(event `self.ReceiveBeginPlay`)

(event `self.K2_PostLogin`
  (params (NewPlayer :type "PlayerController Object Reference"))
  (`parent.K2_PostLogin` NewPlayer))

(event `Event_Assign_To_Team`)

(fn `UserConstructionScript`)